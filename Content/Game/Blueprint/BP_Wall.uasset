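; BP_Wall is a wall actor that emits sound from its Audio component within a configurable box-shaped area.
; On BeginPlay it sets box attenuation from the BoxSound extents and FallOffDistance, then starts playback.
; Every Tick it runs a zero-length box trace with the same extents at the Audio component, using only its debug drawing to show the sound volume.
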(event `self.ReceiveTick`
  (params (DeltaSeconds :type "Float (single-precision)"))
  (bind _audio (`self.Audio`))
  (bind _returnvalue (`SceneComponent.K2_GetComponentLocation` _audio))
  (`KismetSystemLibrary.BoxTraceSingle` :`Start` _returnvalue :`End` _returnvalue :`HalfSize` (`KismetMathLibrary.MakeVector` (`self.BoxSoundX`) (`self.BoxSoundY`) (`self.BoxSoundZ`)) :`Orientation` (`SceneComponent.K2_GetComponentRotation` _audio) :`TraceChannel` "TraceTypeQuery1" :`DrawDebugType` "ForDuration" :`DrawTime` 2.0))

(event `self.ReceiveBeginPlay`
  (`AudioComponent.AdjustAttenuation` (`self.Audio`) (make `SoundAttenuationSettings` true true false false false false false true false false false false false true "SPATIALIZATION_Default" null 0.0 (struct :`EditorCurveData` (struct :`DefaultValue` 3.4028234663852886e+38 :`PreInfinityExtrap` "RCCE_Constant" :`PostInfinityExtrap` "RCCE_Constant")) (struct :`EditorCurveData` (struct :`DefaultValue` 3.4028234663852886e+38 :`PreInfinityExtrap` "RCCE_Constant" :`PostInfinityExtrap` "RCCE_Constant")) "Linear" "ECC_Visibility" "Linear" "Linear" 0.0 0.0 "OmniDirectional" 200.0 3000.0 6000.0 20000.0 20000.0 0.0 0.0 30.0 60.0 1.0 1.0 1.0 1.0 1.0 1.0 1.0 1.0 20000.0 1.0 0.1 0.3 0.95 400.0 4000.0 0.0 1.0 1.0 400.0 4000.0 1.0 (struct :`EditorCurveData` (struct :`DefaultValue` 3.4028234663852886e+38 :`PreInfinityExtrap` "RCCE_Constant" :`PostInfinityExtrap` "RCCE_Constant")) _ (struct :`EditorCurveData` (struct :`DefaultValue` 3.4028234663852886e+38 :`PreInfinityExtrap` "RCCE_Constant" :`PostInfinityExtrap` "RCCE_Constant")) (struct) "Linear" "Box" "Continues" -60.0 (`KismetMathLibrary.MakeVector` (`self.BoxSoundX`) (`self.BoxSoundY`) (`self.BoxSoundZ`)) 0.0 (`self.FallOffDistance`)))
  (`AudioComponent.Play` (`self.Audio`) 0.0))

(fn `UserConstructionScript`)