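; BP_Balle is a bullet that hits the first-person character and pans its MetaSound relative to the player.
; It binds to the character's location event on BeginPlay.
; Each update dots the player's forward and right vectors with the direction to the bullet's ForwardVector component, feeding front/rear and left/right pan parameters.
; Box overlap calls Hit on the character, or destroys the bullet for any other actor.
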(event `self.ReceiveBeginPlay`
  (bind _returnvalue (`GameplayStatics.GetActorOfClass` "/Game/FirstPerson/Blueprints/BP_FirstPersonCharacter.BP_FirstPersonCharacter_C"))
  (add `/Game/FirstPerson/Blueprints/BP_FirstPersonCharacter.PlayerLocation` _returnvalue (delegate `PlayerLocation`)))

(event `PlayerLocation`
  (params (Location :type "Vector Structure") (Forward :type "Vector Structure") (Right :type "Vector Structure"))
  (bind _metasoundbullet (`self.MetaSoundBullet`))
  (bind _returnvalue (`KismetMathLibrary.Normal` (- (`SceneComponent.K2_GetComponentLocation` (`self.ForwardVector`)) Location)))
  (set `self.A` (`KismetMathLibrary.Dot_VectorVector` Forward _returnvalue))
  (set `self.B` (`KismetMathLibrary.Dot_VectorVector` Right _returnvalue))
  (`AudioParameterControllerInterface.SetFloatParameter` _metasoundbullet "Left <> Right  PAN" (`self.B`))
  (`AudioParameterControllerInterface.SetFloatParameter` _metasoundbullet "Front <> Rear PAN" (`self.A`)))

(event `self.Box.OnComponentBeginOverlap`
  (params (OverlappedComponent :type "PrimitiveComponent Object Reference") (OtherActor :type "Actor Object Reference") (OtherComp :type "PrimitiveComponent Object Reference") (OtherBodyIndex :type Integer) (bFromSweep :type Boolean) (SweepResult :type "HitResult Structure (by ref)"))
  (bind _asbp_first_person_character (cast `/Game/FirstPerson/Blueprints/BP_FirstPersonCharacter` OtherActor)
    (:`then`
      (`/Game/FirstPerson/Blueprints/BP_FirstPersonCharacter.Hit` _asbp_first_person_character))
    (:`CastFailed`
      (`self.K2_DestroyActor`))))

(fn `UserConstructionScript`)