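; BP_Changelevel1 is an end-of-level trigger that quits the game once every turret in its array is gone.
; KillTurret polls TurretArray on a short delay loop, pruning invalid entries in reverse order until it is empty, then sets TourelleFinish.
; Overlapping the Box while that flag is set plays the robot's closing dialogue, waits, then calls QuitGame; despite the asset's name, no level is loaded.
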(event `self.Box.OnComponentBeginOverlap`
  (params (OverlappedComponent :type "PrimitiveComponent Object Reference") (OtherActor :type "Actor Object Reference") (OtherComp :type "PrimitiveComponent Object Reference") (OtherBodyIndex :type Integer) (bFromSweep :type Boolean) (SweepResult :type "HitResult Structure (by ref)"))
  (if (`self.TourelleFinish?`)
    (`GameplayStatics.PlaySound2D` "/Game/Sound/SoundEffect/Dialogue/DialogueRobotFin.DialogueRobotFin" 1.0 1.0 0.0 null null)
    (`KismetSystemLibrary.Delay` 6.0)
    (`KismetSystemLibrary.QuitGame` null "Quit")))

(event `KillTurret`
  (bind (_arrayindex _arrayelement) (`/Engine/EditorBlueprintResources/StandardMacros.ReverseForEachLoop` (`self.TurretArray`) :!label _label)
    (:`LoopBody`
      (`/Engine/EditorBlueprintResources/StandardMacros.IsValid` _arrayelement
        (:`Is Not Valid`
          (`KismetArrayLibrary.Array_Remove` (`self.TurretArray`) _arrayindex))))
    (:`Completed`
      (if (`KismetArrayLibrary.Array_IsEmpty` (`self.TurretArray`))
        (set `self.TourelleFinish?` true)
        (else
          (`KismetSystemLibrary.Delay` 0.5)
          (goto _label))))))

(fn `UserConstructionScript`)